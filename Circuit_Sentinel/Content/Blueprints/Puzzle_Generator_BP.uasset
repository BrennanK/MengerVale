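; Puzzle generator actor that builds a randomized node-and-edge layout and spawns it as Node_BP actors.
; The construction script records edges linking early nodes to start index 0, later nodes to random unused predecessors, and final nodes to end index NodeCount + 1.
; It places nodes at random Y with non-decreasing random X.
; BeginPlay scales PuzzleArea and spawns an indexed node at each stored transform, leaving EdgeSet unused here.
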(event `self.ReceiveBeginPlay`
  (`SceneComponent.SetRelativeScale3D` (`self.Puzzle Area`) (10.0 10.0 1.0))
  (for (_array_element _array_index) (`self.Node Spawn Transform`)
    (bind _returnvalue (`|SpawnActorFromClass` "/Game/Blueprints/Node_BP.Node_BP_C" _array_element "Undefined" "MultiplyWithRoot" null null))
    (set `/Game/Blueprints/Node_BP.Node Index` _array_index _returnvalue)))

(fn `UserConstructionScript`
  (locals (`Last X Coord` :type "Float (double-precision)") (`Used Nodes Count` :type Integer) (`Next Node Choices` :type "Set of Integer") (`Current Node` :type Integer))
  (for _index (range 1 (+ (`self.Node Count`) 1))
    (bind _returnvalue (> (- (`self.Node Count`) (`self.Node Removal Count`)) _index))
    (bind _returnvalue_2 (> _index (+ (`self.Node Removal Count`) 1)))
    (if (and _returnvalue _returnvalue_2)
      (bind _result (`BlueprintSetLibrary.Set_ToArray` (`self.Unused Nodes`) :!label _label))
      (bind _output_get (set `self.Node To Remove` (`KismetArrayLibrary.Array_Random` _result)))
      (`BlueprintSetLibrary.Set_Remove` (`self.Unused Nodes`) _output_get)
      (`BlueprintMapLibrary.Map_Add` (`self.Edge Set`) (`self.Node To Remove`) _index)
      (elif _returnvalue_2
        (goto _label)
        (else
          (`BlueprintMapLibrary.Map_Add` (`self.Edge Set`) 0 _index))))
    (if _returnvalue
      (`BlueprintSetLibrary.Set_Add` (`self.Unused Nodes`) _index)
      (else
        (`BlueprintMapLibrary.Map_Add` (`self.Edge Set`) _index (+ (`self.Node Count`) 1))))
    (bind _output_get_2 (set `local.Last X Coord` (`KismetMathLibrary.RandomFloatInRange` (`local.Last X Coord`) (`self.X size`))))
    (`KismetArrayLibrary.Array_Add` (`self.Node Spawn Transform`) (`KismetMathLibrary.MakeTransform` (`KismetMathLibrary.MakeVector` _output_get_2 (`KismetMathLibrary.RandomFloatInRange` 0.0 (`self.Y size`)))))))