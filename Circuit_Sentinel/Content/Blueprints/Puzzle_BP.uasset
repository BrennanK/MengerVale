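; Cable-network puzzle actor that tests whether the player's network survives random node failures, advancing the day or ending the game.
; BeginPlay, standing in for the construction script, uses the day's data-table row to generate redundant paths between two primary nodes, then spawns them minus some cables.
; On player exit, it destroys random intermediate nodes and graph-searches neighbor sets for a surviving link.
; Success reloads the map on the next day; failure opens the title menu.
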(event `Construct Replacement`
  (bind _returnvalue (- (`self.Y size`) 200.0))
  ;[1 1 1] For whatever reason, the constructionScript is not performing anything inside it in the build. This is a replacement of that function for the time being. Maybe it's not calling the overridden script and calling the default on
  (`SceneComponent.SetWorldScale3D` (`self.Puzzle Area`) (`KismetMathLibrary.MakeVector` (`self.X size`) (`self.Y size`) 1.0))
  (bind _asgame_instance_bp (cast `/Game/Blueprints/Game_Instance_BP` (`GameplayStatics.GetGameInstance`))
    (:`then`
      (bind _returnvalue_2 (`KismetStringLibrary.Conv_IntToString` (`/Game/Blueprints/Game_Instance_BP.Day Num` _asgame_instance_bp)))
      (`KismetSystemLibrary.PrintString` _returnvalue_2 true true (struct :`R` 1.0 :`B` 0.032916 :`A` 1.0) 60.0))
    (:`CastFailed`
      (`KismetSystemLibrary.PrintString` "Cast to game instance failed")))
  (bind _returnvalue_3 (`|GetDataTableRow` "/Game/Blueprints/Day_Num_Param.Day_Num_Param" (`KismetStringLibrary.Conv_StringToName` _returnvalue_2))
    (:`then`
      (bind (_totalnodes _numnodestoremove _extrasparecables _numcablesremoved) (break `/Game/Blueprints/Puzzle_Generation_Param` _returnvalue_3))
      (set `self.Node Count` _totalnodes)
      (set `self.Node Removal Count` _numnodestoremove)
      (bind _output_get (set `self.Num Cables Removed` _numcablesremoved))
      (set `self.Spare Cables` (+ _output_get _extrasparecables))
      (for _index (range 1 (+ (`self.Node Count`) 1))
        (bind _returnvalue_4 (> (- (`self.Node Count`) (`self.Node Removal Count`)) _index))
        (bind _returnvalue_5 (> _index (+ (`self.Node Removal Count`) 1)))
        (if (and _returnvalue_4 _returnvalue_5)
          (bind _result (`BlueprintSetLibrary.Set_ToArray` (`self.Unused Nodes`) :!label _label))
          (bind _output_get_2 (set `self.Node To Remove` (`KismetArrayLibrary.Array_Random` _result)))
          (`BlueprintSetLibrary.Set_Remove` (`self.Unused Nodes`) _output_get_2)
          (`KismetArrayLibrary.Array_Add` (`self.Solved Edge Set`) (make `/Game/Blueprints/2D_Int` (`self.Node To Remove`) _index))
          (elif _returnvalue_5
            (goto _label)
            (else
              (`KismetArrayLibrary.Array_Add` (`self.Solved Edge Set`) (make `/Game/Blueprints/2D_Int` 0 _index)))))
        (if _returnvalue_4
          (`BlueprintSetLibrary.Set_Add` (`self.Unused Nodes`) _index)
          (else
            (`KismetArrayLibrary.Array_Add` (`self.Solved Edge Set`) (make `/Game/Blueprints/2D_Int` _index (+ (`self.Node Count`) 1)))))
        (`KismetArrayLibrary.Array_Add` (`self.Node Spawn Coords`) (`KismetMathLibrary.MakeVector` (* (- (`self.X size`) 300.0) (`KismetMathLibrary.RandomFloatInRange` -1.0 1.0)) (- (* (/ (`KismetMathLibrary.RandomFloatInRange` (`KismetMathLibrary.Conv_IntToDouble` (- _index 1)) (`KismetMathLibrary.Conv_IntToDouble` _index)) (`self.Node Count`)) 2.0 _returnvalue) _returnvalue)))))))

(event `self.ReceiveBeginPlay`
  (bind _nodelist (`self.NodeList`))
  (`self.Construct Replacement`)
  ;[1 1 1] Spawn First Primary Node and add it to list (Index 0)
  (bind _returnvalue (`|SpawnActorFromClass` "/Game/Blueprints/Primary_Node_BP.Primary_Node_BP_C" (`KismetMathLibrary.MakeTransform` (`KismetMathLibrary.TransformLocation` (`self.GetTransform`) (`KismetMathLibrary.MakeVector` 0.0 (- 200.0 (`self.Y size`))))) "AdjustIfPossibleButAlwaysSpawn" "MultiplyWithRoot" null null))
  (bind _output_get (set `self.Node Pointer` _returnvalue))
  (bind _returnvalue_2 (`KismetArrayLibrary.Array_Add` (`self.NodeList`) _output_get))
  (set `/Game/Blueprints/Node_BP.Index` _returnvalue_2 _returnvalue)
  ;[1 1 1] Spawn intermediate nodes (indexed from 1 to Node count)
  (for _array_element (`self.Node Spawn Coords`)
    (bind _returnvalue_3 (`|SpawnActorFromClass` "/Game/Blueprints/Intermediate_Node_BP.Intermediate_Node_BP_C" (`KismetMathLibrary.MakeTransform` (`KismetMathLibrary.TransformLocation` (`SceneComponent.GetRelativeTransform` (`self.DefaultSceneRoot`)) _array_element)) "Undefined" "MultiplyWithRoot" null null))
    (bind _output_get_2 (set `self.Node Pointer` _returnvalue_3))
    (bind _returnvalue_4 (`KismetArrayLibrary.Array_Add` (`self.NodeList`) _output_get_2))
    (set `/Game/Blueprints/Node_BP.Index` _returnvalue_4 _returnvalue_3))
  ;[1 1 1] Spawn second primary node (indexed at Node count + 1)
  (bind _returnvalue_5 (`|SpawnActorFromClass` "/Game/Blueprints/Primary_Node_BP.Primary_Node_BP_C" (`KismetMathLibrary.MakeTransform` (`KismetMathLibrary.TransformLocation` (`SceneComponent.GetRelativeTransform` (`self.DefaultSceneRoot`)) (`KismetMathLibrary.MakeVector` 0.0 (- (`self.Y size`) 200.0)))) "Undefined" "MultiplyWithRoot" null null))
  (bind _output_get_3 (set `self.Node Pointer` _returnvalue_5))
  (bind _returnvalue_6 (`KismetArrayLibrary.Array_Add` (`self.NodeList`) _output_get_3))
  (set `/Game/Blueprints/Node_BP.Index` _returnvalue_6 _returnvalue_5)
  (bind _output_get_4 (set `self.Edge Set` (`self.Solved Edge Set`)))
  (for _ (range 1 (+ (`self.Num Cables Removed`) 1))
    (`KismetArrayLibrary.Array_RemoveItem` _output_get_4 (`KismetArrayLibrary.Array_Random` _output_get_4)))
  (for _array_element_2 (`self.Edge Set`)
    (bind (_start _end) (break `/Game/Blueprints/2D_Int` _array_element_2))
    (`self.Create new Connection` self (`|GetArrayItem` _nodelist _start) (`|GetArrayItem` _nodelist _end))
    (`KismetSystemLibrary.PrintText` (`KismetTextLibrary.Conv_StringToText` (`KismetStringLibrary.Concat_StrStr` "(" (`KismetStringLibrary.Conv_IntToString` _start) ", " (`KismetStringLibrary.Conv_IntToString` _end) ")")) true true (struct :`R` 0.372372 :`B` 1.0 :`A` 1.0) 180.0))
  (`|ExecutionSequence`
    (:`then_0`
      (bind _asbp_third_person_character (cast `/Game/ThirdPerson/Blueprints/BP_ThirdPersonCharacter` (`GameplayStatics.GetPlayerCharacter` 0)))
      (set `self.Player Ref` _asbp_third_person_character)
      (add `self.On Player Win` (delegate `On Player Win_Event`)))
    (:`then_1`
      (add `self.On Player Lose` (delegate `On Player Lose_Event`)))
    (:`then_2`
      (add `self.On Player Exit` (delegate `On Player Exit_Event`)))))

(event `On Player Win_Event`
  (`/Game/ThirdPerson/Blueprints/BP_ThirdPersonCharacter.On Win` (`self.Player Ref`))
  (`KismetSystemLibrary.Delay` 5.0)
  (bind _asgame_instance_bp (cast `/Game/Blueprints/Game_Instance_BP` (`GameplayStatics.GetGameInstance`)))
  (bind _result (`/Engine/EditorBlueprintResources/StandardMacros.IncrementInt` (`/Game/Blueprints/Game_Instance_BP.Day Num` _asgame_instance_bp))
    (:`  `
      (set `/Game/Blueprints/Game_Instance_BP.Day Num` _result _asgame_instance_bp)
      (`GameplayStatics.OpenLevelBySoftObjectPtr` "/Game/PlayTest_1_Map.PlayTest_1_Map"))))

(event `self.ReceiveActorBeginOverlap`
  (params (OtherActor :type "Actor Object Reference")))

(event `self.ReceiveTick`
  (params (DeltaSeconds :type "Float (single-precision)")))

(event `self.ReceiveActorEndOverlap`
  (params (OtherActor :type "Actor Object Reference"))
  (bind _player_ref (`self.Player Ref`))
  (if (== OtherActor _player_ref)
    (`/Game/ThirdPerson/Blueprints/BP_ThirdPersonCharacter.On Puzzle Exit_Event` _player_ref)
    (else
      (`KismetSystemLibrary.PrintString` (`KismetSystemLibrary.GetDisplayName` OtherActor) true true (struct :`R` 1.0 :`B` 0.46345 :`A` 1.0) 60.0))))

(event `On Player Lose_Event`
  (`/Game/ThirdPerson/Blueprints/BP_ThirdPersonCharacter.On Lose` (`self.Player Ref`))
  (`KismetSystemLibrary.Delay` 5.0)
  (bind _asgame_instance_bp (cast `/Game/Blueprints/Game_Instance_BP` (`GameplayStatics.GetGameInstance`)))
  (`/Game/Blueprints/Game_Instance_BP.On Game Over_Event` _asgame_instance_bp)
  (set `PlayerController.bShowMouseCursor` true (`GameplayStatics.GetPlayerController` 0))
  (`GameplayStatics.OpenLevel` "Title_Menu"))

(event `On Player Exit_Event`
  (`KismetSystemLibrary.PrintText` "On Player Exit Called" true true (struct :`G` 0.66 :`B` 1.0 :`A` 1.0) 60.0)
  (`self.Destroy Nodes`)
  (for _array_element (`self.NodeList`)
    (bind _result (`BlueprintSetLibrary.Set_ToArray` (`/Game/Blueprints/Node_BP.Neighbors` _array_element)))
    (for _array_element_2 _result
      (`KismetSystemLibrary.PrintString` (`KismetSystemLibrary.GetDisplayName` _array_element_2) true true (struct :`R` 1.0 :`B` 0.350625 :`A` 1.0) 180.0)))
  (bind _successful (`self.Check Connectivity`))
  (`KismetSystemLibrary.PrintString` (`KismetStringLibrary.Conv_BoolToString` _successful) true true (struct :`R` 1.0 :`G` 0.102151 :`A` 1.0) 30.0)
  (if _successful
    (`self.On Player Win`)
    (else
      (`self.On Player Lose`))))

(fn `Check Connectivity`
  (returns (Successful :type Boolean))
  (locals (Stack :type "Set of /Game/Blueprints/Node_BP Object Reference") (Visited :type "Array of /Game/Blueprints/Node_BP Object Reference") (`Current Node` :type "/Game/Blueprints/Node_BP Object Reference") (Success :type Boolean))
  (bind _stack (`local.Stack`))
  (bind _output (`|GetArrayItem` (`self.NodeList`)))
  (for _array_element (`self.NodeList`)
    (if (`BlueprintSetLibrary.Set_IsEmpty` (`/Game/Blueprints/Node_BP.Neighbors` _array_element))
      (return false)))
  (`KismetArrayLibrary.Array_Add` (`local.Visited`) _output)
  (bind _result (`BlueprintSetLibrary.Set_ToArray` (`/Game/Blueprints/Node_BP.Neighbors` _output)))
  (`BlueprintSetLibrary.Set_AddItems` _stack _result)
  (while (`BlueprintSetLibrary.Set_IsNotEmpty` _stack)
    (bind _result_2 (`BlueprintSetLibrary.Set_ToArray` (`local.Stack`)))
    (bind _output_2 (`|GetArrayItem` _result_2))
    (`KismetArrayLibrary.Array_Add` (`local.Visited`) _output_2)
    (bind _result_3 (`BlueprintSetLibrary.Set_ToArray` (`/Game/Blueprints/Node_BP.Neighbors` _output_2)))
    (`BlueprintSetLibrary.Set_Remove` (`local.Stack`) _output_2)
    (for _array_element_2 _result_3
      (if (== (`/Game/Blueprints/Node_BP.Index` _array_element_2) (+ (`self.Node Count`) 1))
        (return true)
        (elif (not (`KismetArrayLibrary.Array_Contains` (`local.Visited`) _array_element_2))
          (`BlueprintSetLibrary.Set_Add` (`local.Stack`) _array_element_2)))))
  (return false))

(fn `Create new Connection`
  (params (`Node 1` :type "/Game/Blueprints/Node_BP Object Reference") (`Node 2` :type "/Game/Blueprints/Node_BP Object Reference"))
  (bind _node_1 (`local.Node 1`))
  (bind _node_2 (`local.Node 2`))
  (bind _cable_connection (`/Game/Blueprints/Node_BP.Cable Connection` `Node 2`))
  (bind _nodelist (`self.NodeList`))
  (bind _returnvalue (`|SpawnActorFromClass` "/Game/Blueprints/Cabling_BP.Cabling_BP_C" (`SceneComponent.K2_GetComponentToWorld` (`/Game/Blueprints/Node_BP.Cable Connection` `Node 1`)) "Undefined" "MultiplyWithRoot" null null))
  (bind _cable (`/Game/Blueprints/Cabling_BP.Cable` _returnvalue))
  (set `CableComponent.CableLength` (* (`self.GetDistanceTo` _returnvalue `Node 2`) 0.5) _cable)
  (`CableComponent.SetAttachEndToComponent` _cable _cable_connection "None")
  (`NiagaraComponent.SetVariableVec3` (`/Game/Blueprints/Cabling_BP.Niagara` _returnvalue) "Beam End" (`SceneComponent.K2_GetComponentLocation` _cable_connection))
  (`BlueprintMapLibrary.Map_Add` (`self.Cable List`) (make `/Game/Blueprints/2D_Int` (`KismetArrayLibrary.Array_Find` _nodelist `Node 1`) (`KismetArrayLibrary.Array_Find` _nodelist `Node 2`)) _returnvalue)
  (`BlueprintSetLibrary.Set_Add` (`/Game/Blueprints/Node_BP.Neighbors` _node_1) _node_2)
  (`BlueprintSetLibrary.Set_Add` (`/Game/Blueprints/Node_BP.Neighbors` _node_2) _node_1)
  (`BlueprintSetLibrary.Set_Add` (`/Game/Blueprints/Node_BP.Incident Cables` (`local.Node 1`)) _returnvalue)
  (`BlueprintSetLibrary.Set_Add` (`/Game/Blueprints/Node_BP.Incident Cables` (`local.Node 2`)) _returnvalue))

(fn `Destroy Nodes`
  (locals (`Node To Destroy` :type "/Game/Blueprints/Node_BP Object Reference"))
  (bind _nodelist (`self.NodeList`))
  (bind _cable_list (`self.Cable List`))
  (for _ (range 1 (+ (`self.Node Removal Count`) 1))
    (bind _output_get (set `local.Node To Destroy` (`|GetArrayItem` _nodelist (`KismetMathLibrary.RandomIntegerInRange` 1 (- (`KismetArrayLibrary.Array_Length` _nodelist) 2)))))
    (for _array_element (`self.Edge Set`)
      (bind (_start _end) (break `/Game/Blueprints/2D_Int` _array_element))
      (bind _index (`/Game/Blueprints/Node_BP.Index` _output_get))
      (if (or (== _start _index) (== _end _index))
        (`self.K2_DestroyActor` (`BlueprintMapLibrary.Map_Find` _cable_list _array_element))
        (`BlueprintMapLibrary.Map_Remove` _cable_list _array_element)
        (`KismetArrayLibrary.Array_RemoveItem` (`self.Edge Set`) _array_element)))
    (for _array_element_2 (`self.NodeList`)
      (`BlueprintSetLibrary.Set_Remove` (`/Game/Blueprints/Node_BP.Neighbors` _array_element_2) _output_get))
    (`KismetSystemLibrary.PrintString` (`KismetSystemLibrary.GetDisplayName` _output_get) true true (struct :`R` 1.0 :`G` 0.894209 :`A` 1.0) 180.0)
    (`KismetArrayLibrary.Array_RemoveItem` (`self.NodeList`) _output_get)
    (`self.K2_DestroyActor` _output_get)))

(fn `Get Node Removal Count`
  (returns (Nodes :type Integer))
  (return (`self.Node Removal Count`)))

(fn `UserConstructionScript`
  (locals (Section :type "Float (double-precision)") (`Used Nodes Count` :type Integer) (`Next Node Choices` :type "Set of Integer") (`Current Node` :type Integer)))