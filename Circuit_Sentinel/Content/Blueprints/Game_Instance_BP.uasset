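; Game instance that tracks whether a run is in progress and the current day number for a night-survival game.
; The game-start event sets the run active at day one.
; The game-over event ends the run and saves the day count minus one as MostNightsSurvived in Slot1, loading or creating a Saved_Game_BP.
; The stored value is overwritten without comparison to the previous record.
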(event `On Game Start_Event`
  (set `self.Game In Progress` true)
  (set `self.Day Num` 1))

(event `On Game Over_Event`
  (bind _returnvalue (- (`self.Day Num`) 1))
  (set `self.Game In Progress` false)
  (bind _returnvalue_2 (`GameplayStatics.DoesSaveGameExist` "Slot1"))
  (if _returnvalue_2
    (bind _returnvalue_3 (`GameplayStatics.LoadGameFromSlot` "Slot1"))
    (bind _assaved_game_bp (cast `/Game/Blueprints/Saved_Game_BP` _returnvalue_3)
      (:`then`
        (set `/Game/Blueprints/Saved_Game_BP.Most Nights Survived` _returnvalue _assaved_game_bp)
        (`GameplayStatics.SaveGameToSlot` _assaved_game_bp "Slot1"))
      (:`CastFailed`
        (`KismetSystemLibrary.PrintString` "Cast to Saved_Game_BP failed" true true (struct :`G` 0.338542 :`B` 0.133699 :`A` 1.0))))
    (else
      (bind _returnvalue_4 (`GameplayStatics.CreateSaveGameObject` "/Game/Blueprints/Saved_Game_BP.Saved_Game_BP_C"))
      (set `/Game/Blueprints/Saved_Game_BP.Most Nights Survived` _returnvalue _returnvalue_4)
      (`GameplayStatics.SaveGameToSlot` _returnvalue_4 "Slot1"))))