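; Skylight Blueprint intended to fade light intensity as a timer runs down, though the fade is currently disconnected.
; SetTotalTime stores the timer's full duration, while UpdateSkylightIntensity receives the remaining time but does nothing.
; An unreachable chain lerps LightComponent intensity from final to initial by the fraction of time remaining and prints the result for debugging.
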(event `/Game/Blueprints/Skylight_BPI.Update Skylight Intensity`
  (params (`Time Remaining` :type "Float (double-precision)")))

(event `/Game/Blueprints/Skylight_BPI.Set Total Time`
  (params (Time :type "Float (double-precision)"))
  (set `self.Total Time` Time))

(fn `UserConstructionScript`)