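; Tutorial manager actor that steps the player through the tutorial level by advancing panels in a TutorialPanel widget.
; It spawns movement triggers one after another at preset transforms, handing each a self-reference, and advances once three movement steps are counted.
; The puzzle step spawns Puzzle_BP at the manager's transform and notifies the player character.
; Tick then watches the player's spare cables and advances once when none remain.
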(event `self.ReceiveBeginPlay`
  (`|ExecutionSequence`
    (:`then_0`
      (bind _returnvalue (`|CreateWidget` "/Game/Levels/Tutoriallevel_actors/TutorialPanel_Widget.TutorialPanel_Widget_C"))
      (bind _output_get (set `self.Panelref` _returnvalue))
      (`UserWidget.AddToViewport` _output_get 0)
      (set `self.CurrentIndex` -1)
      (`self.nextTutorial`)
      (`self.CreateMovementTrigger`))
    (:`then_1`
      (bind _returnvalue_2 (`GameplayStatics.GetActorOfClass` "/Game/ThirdPerson/Blueprints/BP_ThirdPersonCharacter.BP_ThirdPersonCharacter_C"))
      (set `self.PlayerRef` _returnvalue_2))))

(event `self.ReceiveTick`
  (params (DeltaSeconds :type "Float (single-precision)"))
  (if (`self.DoneMovement`)
    (`KismetSystemLibrary.Delay` 1.0)
    (bind _spare_cables (`/Game/Blueprints/BPI_ThirdPersonCharacter.Get Spare Cables` (`self.PlayerRef`)))
    (if (== _spare_cables 0)
      (`/Engine/EditorBlueprintResources/StandardMacros.DoOnce` false
        (:`Completed`
          (`self.nextTutorial`))))))

(fn ` AddMovementTutorial`
  (bind _result (`/Engine/EditorBlueprintResources/StandardMacros.IncrementInt` (`self.MovementCount`))
    (:`  `
      (bind _output_get (set `self.MovementCount` _result))
      (if (>= _output_get 3)
        (`self.nextTutorial`)
        (else
          (`self.CreateMovementTrigger`))))))

(fn `CreateMovementTrigger`
  (bind _returnvalue (`|SpawnActorFromClass` "/Game/Levels/Tutoriallevel_actors/MovementTrigger_BP.MovementTrigger_BP_C" (`|GetArrayItem` (`self.MovementTransforms`) (`self.MovementCount`)) "Undefined" "MultiplyWithRoot" null null))
  (`/Game/Levels/Tutoriallevel_actors/MovementTrigger_BP.SetManagerRef` _returnvalue self))

(fn `nextTutorial`
  (bind _result (`/Engine/EditorBlueprintResources/StandardMacros.IncrementInt` (`self.CurrentIndex`))
    (:`  `
      (bind _output_get (set `self.CurrentIndex` _result))
      (`/Game/Levels/Tutoriallevel_actors/TutorialPanel_Widget.ActivePanel` (`self.Panelref`) _output_get)
      (if (== _output_get 1)
        (`|SpawnActorFromClass` "/Game/Blueprints/Puzzle_BP.Puzzle_BP_C" (`self.GetTransform`) "Undefined" "MultiplyWithRoot" null null)
        (bind _returnvalue (`GameplayStatics.GetActorOfClass` "/Game/ThirdPerson/Blueprints/BP_ThirdPersonCharacter.BP_ThirdPersonCharacter_C"))
        (`/Game/ThirdPerson/Blueprints/BP_ThirdPersonCharacter.OnPuzzleCreate` _returnvalue)
        (set `self.DoneMovement` true)))))

(fn `SetMissionText`
  (bind _currentindex (`self.CurrentIndex`))
  (if (== _currentindex 0)
    (`TextRenderComponent.K2_SetText` (`self.MissionText`) (`KismetTextLibrary.Conv_StringToText` "Move to Nodes"))
    (elif (== _currentindex 1)
      (`TextRenderComponent.K2_SetText` (`self.MissionText`) (`KismetTextLibrary.Conv_StringToText` "Move to Nodes")))))

(fn `UserConstructionScript`)